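; BP_ActivateableDoor_1 is a door actor that moves its Door component between a starting and a destination transform.
; The construction script captures the Door's current relative transform as the starting pose.
; It overrides the parent's OnUpdateTimeline, using the supplied alpha to lerp the Door's relative transform toward DoorDestinationTransform without sweeping.
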(event `self.ReceiveBeginPlay`
  (`parent.ReceiveBeginPlay`))

(fn `OnUpdateTimeline`
  (params (Alpha :type "Float (double-precision)"))
  (`parent.OnUpdateTimeline` Alpha)
  (`SceneComponent.K2_SetRelativeTransform` (`self.Door`) (`KismetMathLibrary.TLerp` (`self.DoorStartingTransform`) (`self.DoorDestinationTransform`) (`local.Alpha`)) false false))

(fn `UserConstructionScript`
  (`parent.UserConstructionScript`)
  (set `self.DoorStartingTransform` (`SceneComponent.GetRelativeTransform` (`self.Door`))))