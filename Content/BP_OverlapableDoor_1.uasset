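; An overlap-triggered door that opens when a Character enters its sphere and closes once no Characters remain in range.
; Sphere begin and end overlap events both call CheckforOverlappingActors, which compares Character presence against the door's active state.
; On a mismatch it toggles the door through InteractableComp.StartInteraction with the overlapping actor as interactor, requiring that actor to be valid when closing.
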(event `self.Sphere.OnComponentBeginOverlap`
  (params (OverlappedComponent :type "PrimitiveComponent Object Reference") (OtherActor :type "Actor Object Reference") (OtherComp :type "PrimitiveComponent Object Reference") (OtherBodyIndex :type Integer) (bFromSweep :type Boolean) (SweepResult :type "HitResult Structure (by ref)"))
  (`self.CheckforOverlappingActors` (`self.Sphere`) OtherActor))

(event `self.Sphere.OnComponentEndOverlap`
  (params (OverlappedComponent :type "PrimitiveComponent Object Reference") (OtherActor :type "Actor Object Reference") (OtherComp :type "PrimitiveComponent Object Reference") (OtherBodyIndex :type Integer))
  (`self.CheckforOverlappingActors` (`self.Sphere`) OtherActor))

(fn `CheckforOverlappingActors`
  (params (Target :type "PrimitiveComponent Object Reference") (Interactor :type "Actor Object Reference"))
  (if (`KismetArrayLibrary.Array_IsValidIndex` (`PrimitiveComponent.GetOverlappingActors` Target "/Script/Engine.Character"))
    (if (not (`self.GetIsActive`))
      (`InteractableComponent.StartInteraction` (`self.InteractableComp`) (`local.Interactor`) :!label _label))
    (elif (`self.GetIsActive`)
      (`local.Interactor`
        (:`then`
          (goto _label))
        (:`else`)))))

(fn `UserConstructionScript`
  (`parent.UserConstructionScript`))