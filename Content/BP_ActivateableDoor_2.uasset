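; BP_ActivateableDoor_2 is a double door that slides or swings its two leaves through a timeline inherited from its parent.
; Construction caches each leaf's starting relative transform, and each timeline update lerps both leaves toward their destination transforms by alpha.
; DisableUserInteraction runs only on authority and, despite its name, toggles the enabled state of the interactor's InteractComponent.
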(fn `DisableUserInteraction`
  (params (Interactor :type "Actor Object Reference"))
  (bind _returnvalue (`self.GetComponentByClass` Interactor "/Script/InteractionSystemPlugin.InteractComponent"))
  (`/Engine/EditorBlueprintResources/ActorMacros.Switch Has Authority`
    (:`Authority`
      (`InteractComponent.SetInteractionEnabled` _returnvalue (not (`InteractComponent.bInteractionEnabled` _returnvalue))))))

(fn `OnUpdateTimeline`
  (params (Alpha :type "Float (double-precision)"))
  (`parent.OnUpdateTimeline` Alpha)
  (`SceneComponent.K2_SetRelativeTransform` (`self.LeftDoor`) (`KismetMathLibrary.TLerp` (`self.LeftDoorStartingTransform`) (`self.LeftDoorDestination`) (`local.Alpha`)) false false)
  (`SceneComponent.K2_SetRelativeTransform` (`self.RightDoor`) (`KismetMathLibrary.TLerp` (`self.RightDoorStartingTransform`) (`self.RightDoorDestination`) (`local.Alpha`)) false false))

(fn `UserConstructionScript`
  (`parent.UserConstructionScript`)
  (set `self.RightDoorStartingTransform` (`SceneComponent.GetRelativeTransform` (`self.RightDoor`)))
  (set `self.LeftDoorStartingTransform` (`SceneComponent.GetRelativeTransform` (`self.LeftDoor`))))